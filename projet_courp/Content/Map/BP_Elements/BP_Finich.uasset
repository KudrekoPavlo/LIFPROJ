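; BP_Finich is the race finish actor that stops the timer once the player has passed enough checkpoints.
; On any actor overlap it reads player state 0 as Player_State_principale, without checking which actor overlapped.
; If the checkpoint count meets the finish requirement, it calls FinirCompter on that state's TimerWidget.
; An unconnected Game Instance version of the same check remains, marked as not valid for online play.
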(event `self.ReceiveActorBeginOverlap`
  (params (OtherActor :type "Actor Object Reference"))
  ; lorsque player fini la course le compteur lui done son temp exact de course
  (bind _asplayer_state_principale (cast `/Game/Menu/Lobby/PlayerState/Player_State_principale` (`GameplayStatics.GetPlayerState` 0)))
  (if (>= (`/Game/Menu/Lobby/PlayerState/Player_State_principale.Compteur_checkpoints` _asplayer_state_principale) (`/Game/Menu/Lobby/PlayerState/Player_State_principale.Checkpoints_for_finish` _asplayer_state_principale))
    (`/Game/VehicleTemplate/UI/UI_Timer.Finir Compter` (`/Game/Menu/Lobby/PlayerState/Player_State_principale.Timer_widget` _asplayer_state_principale))))

(fn `UserConstructionScript`)